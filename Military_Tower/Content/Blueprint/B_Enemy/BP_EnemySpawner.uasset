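; BP_EnemySpawner spawns a group of pooled enemies when play begins.
; On BeginPlay it clears EnemyArray, then loops up to SpawnEnemyMount, pulling each enemy from ACCharacterPool at SpawnLocation with a fixed per-index Y offset.
; Each enemy is cast to BP_EnemyBase_Pool, stored in the array and handed the spawner's spline reference.
; A comment marks the spawn position as still to be revised.
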(event EventBeginPlay
  (Utilities|Array|Clear (Variables|Default|GetEnemyArray))
  (for _index (range 0 (Variables|Default|GetSpawnEnemyMount))
    (bind _array_element (Default|SpawnfromPool (Variables|Default|GetAC_CharacterPool) (Math|Transform|MakeTransform (+ (Variables|Default|GetSpawnLocation) (Math|Vector|MakeVector 0.0 (* _index 450) 0.0)) "0, 0, 0" "1.000000,1.000000,1.000000")))
    (bind _asbp_enemy_base_pool (Utilities|Casting|CastToBP_EnemyBase_Pool _array_element))
    (Utilities|Array|AddUnique (Variables|Default|GetEnemyArray) _asbp_enemy_base_pool)
    (Variables|/Game/Blueprint/B_Enemy/BP_EnemyBase_Pool.BP_EnemyBase_Pool_C|Set%20BP_EnemySpline _asbp_enemy_base_pool (Variables|Default|GetBP%20Enemy%20Spline))))

(fn ConstructionScript)