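; Base enemy pawn that walks along an assigned BPEnemySpline and shows a health bar.
; Movement is a recursive AIMoveTo to random reachable points near each successive spline point, with a short random delay.
; BeginPlay builds a screen-space health widget component and registers the actor as the NSFires Niagara callback.
; AI perception hits and exported particle positions currently only drive debug prints and shapes.
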(event OnPerceptionUpdated(AIPerception)
  (params (UpdatedActors :type Array%20of%20Actor%20Object%20References))
  ;[0 0 0 0.5] AI感知系统
)

(event OnTargetPerceptionUpdated(AIPerception)
  (params (Actor :type Actor%20Object%20Reference) (Stimulus :type AI%20Stimulus%20Structure))
  (bind (_age _expirationage _strength _stimuluslocation _receiverlocation _tag _bsuccessfullysensed) (Utilities|Struct|BreakAIStimulus Stimulus))
  ;[0 0 0 0.5] AI感知系统
  (if _bsuccessfullysensed
    (Development|PrintString (Utilities|GetDisplayName Actor))
    (Rendering|Debug|DrawDebugBox _stimuluslocation "100.000000,100.000000,200.000000" "(R=1.000000,G=0.922429,B=0.000000,A=1.000000)" "0, 0, 0" 1e+01 0.0)))

(event Custom|MoveTo
  ;[0 0 0 0.5] 敌人的移动逻辑
  (Utilities|IsValid (Variables|Default|Get%20BP_EnemySpline)
    (:Is%20Valid
      (AI|AIMoveTo self (.RandomLocation (AI|Navigation|GetRandomReachablePointinRadius (Spline|GetLocationatSplinePoint (Variables|/Game/Blueprint/B_Enemy/BP_EnemySpline.BP_EnemySpline_C|GetSpline (Variables|Default|Get%20BP_EnemySpline)) (Variables|Default|GetSpline%20Point%20Index) "World") 1.5e+02 0 0)) 0 5.0 false
        (:OnSuccess
          (Utilities|FlowControl|Delay (Math|Random|RandomFloatinRange 0.0 0.1))
          (Math|Integer|IncrementInt (Variables|Default|GetSpline%20Point%20Index)
            (:%20%20
              (CallFunction|Moveto))))))
    (:Is%20Not%20Valid
      (Development|PrintString "NO Spline "))))

(event EventBeginPlay
  ;[0 0 0 0.5] 添加生命值组件
  (CallFunction|AddHealthBar)
  (CallFunction|Moveto)
  ;[0 0 0 0.5] niagara回调
  (Class|NiagaraComponent|SetVariableObject (Variables|Default|GetNS_Fires) "BPCallBack" self))

(event EventParticleData
  (params (Data :type Array%20of%20Basic%20Particle%20Data%20Structures) (NiagaraSystem :type Niagara%20System%20Object%20Reference) (SimulationPositionOffset :type Vector%20%28by%20ref%29 :default "0, 0, 0"))
  ;[0 0 0 0.5] Niagara子弹特效碰撞检测
  (for _array_element Data
    (Rendering|Debug|DrawDebugSphere (.Position (Utilities|Struct|BreakBasicParticleData _array_element)) 1e+02 12 "(R=1.000000,G=0.000000,B=0.000000,A=1.000000)" 1.0)))

(fn ConstructionScript)

(fn AddHealthBar
  (bind _returnvalue (AddComponent|AddWidgetComponent false (Math|Transform|MakeTransform "0.000000,0.000000,90.000000" "0, 0, 0" "1.000000,1.000000,1.000000")))
  (Class|WidgetComponent|SetDrawSize _returnvalue "(X=100.000000,Y=20.000000)")
  (Class|WidgetComponent|SetWidgetSpace _returnvalue "Screen")
  (Variables|Default|SetHealthBarWidget _returnvalue)
  (bind _returnvalue_2 (UserInterface|CreateWidget "/Game/Blueprint/B_Widget/EnemyWidget/BPWG_EnemyHealth.BPWG_EnemyHealth_C"))
  (UserInterface|SetWidget (Variables|Default|GetHealthBarWidget) _returnvalue_2)
  (bind _output_get (Variables|Default|SetHealthBar _returnvalue_2))
  (Default|UpdateHealthbar _output_get (Variables|Health|GetCurrentHealth)))

(fn GetEnemyLocation
  (return (Transformation|GetActorLocation)))