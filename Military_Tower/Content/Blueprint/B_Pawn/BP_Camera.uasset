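; BP_Camera is a camera pawn that moves its Sphere component vertically on player input.
; On BeginPlay it creates the BPWG_PlayerUITest widget, adds it to the viewport and passes IshasCommand to its subtitle animation.
; IA_Spring and IA_Spring1 call a shared function that offsets the Sphere's relative Z up or down by MCamerbaseValues.
; That offset scales with the action's ElapsedSeconds rather than frame delta time.
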(event Input|EnhancedActionEvents|EnhancedInputActionIA_Spring1
  (params (ActionValue :type Boolean) (ElapsedSeconds :type Float%20%28double-precision%29) (TriggeredSeconds :type Float%20%28double-precision%29) (InputAction :type Input%20Action%20Object%20Reference :default "/Game/Input/IA_Spring1.IA_Spring1"))
  (CallFunction|VoidUpeerlowerbuffercamera -1.0 ElapsedSeconds))

(event Input|EnhancedActionEvents|EnhancedInputActionIA_Spring
  (params (ActionValue :type Boolean) (ElapsedSeconds :type Float%20%28double-precision%29) (TriggeredSeconds :type Float%20%28double-precision%29) (InputAction :type Input%20Action%20Object%20Reference :default "/Game/Input/IA_Spring.IA_Spring"))
  (CallFunction|VoidUpeerlowerbuffercamera 1.0 ElapsedSeconds))

(event EventBeginPlay
  (bind _returnvalue (UserInterface|CreateWidget "/Game/Blueprint/B_Widget/BPWG_PlayerUITest.BPWG_PlayerUITest_C"))
  (UserInterface|Viewport|AddtoViewport _returnvalue 0)
  (Default|VoidSetSubtitleAnimation _returnvalue (Variables|Default|GetishasCommand)))

(fn ConstructionScript)

(fn VoidUpeerlowerbuffercamera
  (params (camerauporDown :type Float%20%28double-precision%29) (deltaTime :type Float%20%28double-precision%29))
  (bind _sphere (Variables|Default|GetSphere))
  (bind _returnvalue (Transformation|GetRelativeTransform _sphere))
  (Transformation|SetRelativeLocation _sphere (Math|Vector|MakeVector (.x (.location _returnvalue)) (.y (.location _returnvalue)) (+ (.z (.location _returnvalue)) (* camerauporDown (LocalVariables|Getm_camerbaseValues) deltaTime))) false false))