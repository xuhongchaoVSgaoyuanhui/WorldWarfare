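; BFL_GeneralFunction is a function library of general gameplay helpers for timer access and combat math.
; FUGetTimerManager casts the game state to GS_Tower and returns its TimerManager.
; FUDamageCalculationFormula returns the defender's remaining HP, without applying it.
; Its damage divides an attack term boosted by the attacker's Penetrate by the defender's Defense scaled down by that same Penetrate.
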(fn FUGetTimerManager
  ;[0.15 0.15 0.15 0.5] 详细游戏状态
  (bind _asgs_tower (Utilities|Casting|CastToGS_Tower (Game|GetGameState)))
  ;[0.15 0.15 0.15 0.5] 强制明确类型
  (return (Variables|/Game/Gamemode/GS_Tower.GS_Tower_C|GetTimerManager _asgs_tower)))

(fn FUDamageCalculationFormula
  (params (AttackTarget :type Struct%20Attack%20Structure) (DefensiveTarget :type Struct%20Defense%20Structure))
  (bind (_attack _armorpenetration _penetrate) (Utilities|Struct|BreakStruct_Attack AttackTarget))
  (bind (_maxhp _currenthp _armor _defense) (Utilities|Struct|BreakStruct_Defense DefensiveTarget))
  (return (- _currenthp (/ (+ _attack (* _attack (+ _penetrate 1.0))) (* (- 1.0 _penetrate) _defense)))))