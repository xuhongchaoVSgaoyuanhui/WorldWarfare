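; Radar component, apparently for buildings, that detects Enemy objects around its owner and collects them into target groups.
; FURangeDetection clears EnemySorting, runs a debug-drawn multi-sphere trace at the owner's location and passes each hit actor to FUSortiong.
; FUSortiong fills four range-named arrays by count, not measured distance.
; Once an array exceeds 20 entries it advances an index, which is never reset here, and drops that actor.
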(event EventBeginPlay
  (Variables|Default|SetTarget (Components|GetOwner)))

(fn FURangeDetection
  (bind _target (Variables|Default|GetTarget))
  (bind _returnvalue (Transformation|GetActorLocation _target))
  (Variables|Default|SetEnemySorting "")
  (bind (_outhits _returnvalue_2) (Collision|MultiSphereTraceForObjects _returnvalue _returnvalue (Variables|Default|GetNewVar) (LocalVariables|GetEnemy) false 0 "ForDuration"))
  (for _array_element _outhits
    (if _returnvalue_2
      (CallFunction|FUSortiong (.HitActor (Collision|BreakHitResult _array_element))))))

(fn FUSortiong
  (params (TargetIndex :type Actor%20Object%20Reference%20%28by%20ref%29))
  (bind _enemysorting (Variables|Default|GetEnemySorting))
  (bind _enemysortingindex (Variables|Default|GetEnemySortingIndex))
  (bind (_recentgoals _closerangetarget _mediumrangetargetgroup _longdistancetarget) (Utilities|Struct|BreakStruct_Target _enemysorting))
  (bind _returnvalue (Utilities|Select :Index _enemysortingindex :Option%200 _recentgoals :Option%201 _closerangetarget :Option%202 _mediumrangetargetgroup :Option%203 _longdistancetarget))
  (Utilities|IsValid TargetIndex
    (:Is%20Valid
      (if (> (Utilities|Array|Length _returnvalue) 20)
        (Math|Integer|IncrementInt (Variables|Default|GetEnemySortingIndex))
        (else
          (Utilities|Array|Add _returnvalue TargetIndex))))))