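; Targeting component for a building that detects active enemies within range of its owner.
; FU_ActorDetection takes in-use enemies from the enemy manager and, when the circle flag is set, stores those within a 2D distance in EnemiesInRange.
; FU_DirectionConfirmation tests a 45-degree half-angle forward cone by dot product, but only feeds debug print and cone logging, not filtering.
; BeginPlay caches the owner and its AttackComponent.
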(event EventBeginPlay
  (bind _returnvalue (Components|GetOwner))
  (Variables|Default|SetOneSelf _returnvalue)
  (Variables|Default|SetAttackComponent (Utilities|Array|Get(acopy) (Actor|GetComponentsByClass _returnvalue "/Game/Blueprint/BuldingComponent/AttackComponent.AttackComponent_C"))))

(fn FUActorDetection
  (bind _oneself (Variables|Default|GetOneSelf))
  (bind _returnvalue (Transformation|GetActorLocation _oneself))
  (Utilities|Array|Clear (Variables|Default|GetEnemiesInRange))
  (Utilities|Array|Clear (Variables|Default|GetEnemiesInUse))
  (bind _enemymanager (CallFunction|FUGetEnemyManager self))
  (for _array_element (Variables|/Game/Blueprint/B_Enemy/BP_EnemySpawner.BP_EnemySpawner_C|GetEnemyArray _enemymanager)
    (if (Variables|/Game/Blueprint/B_ObjectPool/BP_CharacterPool.BP_CharacterPool_C|GetInUse? _array_element)
      (Utilities|Array|AddUnique (Variables|Default|GetEnemiesInUse) _array_element)))
  (for _array_element_2 (Variables|Default|GetEnemiesInUse)
    (if (< (Math|Vector|Distance2D(Vector) (Math|Vector2D|MakeVector2D (.x (Transformation|GetActorLocation _array_element_2)) (.y (Transformation|GetActorLocation _array_element_2))) (Math|Vector2D|MakeVector2D (.x _returnvalue) (.y _returnvalue))) (Variables|Default|Getdistance))
      (if (Variables|Default|Getbusecircle)
        (Utilities|Array|Add (Variables|Default|GetEnemiesInRange) _array_element_2)
        (Development|PrintString (Utilities|String|ToString(Float) (CallFunction|FUDirectionConfirmation (Math|Conversions|ToVector2D(Vector) (Transformation|GetActorForwardVector _oneself)) (- (Transformation|GetActorLocation _array_element_2) (Transformation|GetActorLocation _oneself)))) true true "(R=1.000000,G=0.787069,B=0.008568,A=1.000000)" 2e+01)))))

(fn FUDirectionConfirmation
  (params (Forward :type Vector%202D%20Structure) (Dir :type Vector%202D%20Structure))
  (bind _oneself (Variables|Default|GetOneSelf))
  (if (> (Math|Vector2D|DotProduct(2D) (Math|Vector2D|Normalize2D Forward) (Math|Vector2D|Normalize2D Dir)) (Math|Trig|Cos(Degrees) 45.0))
    (Class|VisualLoggerKismetLibrary|LogCone 0 (Transformation|GetActorLocation _oneself) (Transformation|GetActorForwardVector _oneself) 5e+03 45.0 "45°夹角检测" "(R=1.000000,G=0.000000,B=0.066378,A=1.000000)" "VisLogBP" false false)
    (return 0.0)))