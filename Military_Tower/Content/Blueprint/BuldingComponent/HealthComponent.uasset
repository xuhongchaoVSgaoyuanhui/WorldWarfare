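; Health component, filed under building components, that holds an Attribute set of max HP, current HP, armor and defense.
; An initializer writes those values by reference, and a getter returns max and current HP.
; TakeDamage runs an external damage formula against Attribute, calling IsAlive when the result is zero or less and HandleDeath otherwise.
; IsAlive and HandleDeath are empty stubs, and BeginPlay does nothing.
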(event EventBeginPlay)

(fn FUTakeDamage
  (params (AttackTarget :type Struct%20Attack%20Structure))
  (if (<= (CallFunction|FUDamageCalculationFormula AttackTarget (Variables|Default|GetAttribute)) 0.0)
    (CallFunction|FUIsAlive)
    (else
      (CallFunction|FUHandleDeath))))

(fn FUInitialAssignmentHealth
  (params (Value%20MaxHealth :type Float%20%28double-precision%29) (Value%20Current%20HP :type Float%20%28double-precision%29) (Value%20Armor :type Integer) (Value%20Defense :type Integer))
  (|SetBy-RefVar (Variables|Default|GetAttribute) (Utilities|Struct|MakeStruct_Defense Value%20MaxHealth Value%20Current%20HP Value%20Armor Value%20Defense)))

(fn FUIsAlive)

(fn FUHandleDeath)

(fn FUReturnHealth
  (bind _attribute (Variables|Default|GetAttribute))
  (bind (_maxhp _currenthp) (Utilities|Struct|BreakStruct_Defense _attribute))
  (return _maxhp _currenthp))