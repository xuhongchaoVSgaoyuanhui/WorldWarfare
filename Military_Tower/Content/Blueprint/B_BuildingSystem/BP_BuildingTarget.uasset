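; Tower placement cursor that shows a building ghost snapped to the grid under the mouse.
; Spawns a hidden BP_BuildingGhost at start; spawn and destroy events only toggle its visibility and set or clear TowerType.
; A looping timer traces under the cursor, moving itself and the ghost in 200-unit steps at zero height.
; The hit actor's Floor tag sets HasBuild (true means blocked) and the grid color through a Material Parameter Collection.
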(event Custom|FollowingMouse
  (bind _returnvalue (Game|GetPlayerController 0))
  (bind _hitresult (Game|Player|GetHitResultUnderCursorbyChannel _returnvalue "TraceTypeQuery1" true))
  (bind (_bblockinghit _binitialoverlap _time _distance _location _impactpoint _normal _impactnormal _physmat _hitactor) (Collision|BreakHitResult _hitresult))
  (bind (_x _y) (Math|Vector|BreakVector _location))
  (bind _returnvalue_2 (+ _x -1e+02))
  (bind _returnvalue_3 (+ _y 1e+02))
  (bind _returnvalue_4 (/ _returnvalue_3 2e+02))
  (bind _returnvalue_5 (/ _returnvalue_2 2e+02))
  (bind _returnvalue_6 (Math|Float|Truncate _returnvalue_4))
  (bind _returnvalue_7 (Math|Float|Truncate _returnvalue_5))
  (bind _returnvalue_8 (* _returnvalue_6 200))
  (bind _returnvalue_9 (* _returnvalue_7 200))
  (bind _returnvalue_10 (Math|Conversions|ToFloat(Integer) _returnvalue_9))
  (bind _returnvalue_11 (Math|Conversions|ToFloat(Integer) _returnvalue_8))
  (bind _returnvalue_12 (Math|Vector|MakeVector _returnvalue_10 _returnvalue_11 0.0))
  ;[0 0 0 0.5] 跟随鼠标
  (Transformation|SetActorLocation (stale EventBeginPlay _returnvalue) _returnvalue_12 false false)
  (Transformation|SetActorLocation _returnvalue_12 false false)
  (Utilities|IsValid _hitactor
    (:Is%20Valid
      ;[0 0 0 0.5] 检测是否能够放置防御塔
      (if (Actor|ActorHasTag _hitactor "Floor")
        (Variables|Default|SetHasBuild false)
        (Rendering|Material|SetVectorParameterValue "/Game/Blueprint/B_BuildingSystem/MPC_BuildingGridColor.MPC_BuildingGridColor" "Color" (Variables|Default|GetEnableColor) :!class /Script/Engine.KismetMaterialLibrary)
        (else
          (Variables|Default|SetHasBuild true)
          (Rendering|Material|SetVectorParameterValue "/Game/Blueprint/B_BuildingSystem/MPC_BuildingGridColor.MPC_BuildingGridColor" "Color" (Variables|Default|GetDisableColor) :!class /Script/Engine.KismetMaterialLibrary))))))

(event Custom|SpawnBuildingGhost
  (params (TowerType :type BP%20Architecture%20Base%20Class%20Reference))
  ;[0 0 0 0.5] 建筑物幽灵
  (Utilities|IsValid (stale EventBeginPlay _returnvalue)
    (:Is%20Valid
      (Rendering|SetActorHiddenInGame (stale EventBeginPlay _returnvalue) false)
      (Variables|Default|SetTowerType TowerType))))

(event Custom|DestroyBuildingGhost
  ;[0 0 0 0.5] 建筑物幽灵
  (Utilities|IsValid (stale EventBeginPlay _returnvalue)
    (:Is%20Valid
      (Rendering|SetActorHiddenInGame (stale EventBeginPlay _returnvalue) true)
      (Variables|Default|SetTowerType 0))))

(event EventBeginPlay
  ;[0 0 0 0.5] 建筑物幽灵
  (bind _returnvalue (Game|SpawnActorfromClass "/Game/Blueprint/B_BuildingSystem/BP_BuildingGhost.BP_BuildingGhost_C" (Math|Transform|MakeTransform "0, 0, 0" "0, 0, 0" "1.000000,1.000000,1.000000") "Undefined" "MultiplyWithRoot" 0 0))
  (Rendering|SetActorHiddenInGame _returnvalue true)
  (Utilities|Time|SetTimerbyEvent (delegate Custom|FollowingMouse) 0.02 true))

(fn ConstructionScript)