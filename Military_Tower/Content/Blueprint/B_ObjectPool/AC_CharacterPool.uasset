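; Actor component that provides an object pool of characters for reuse.
; On BeginPlay it pre-spawns PoolCount characters high above the world origin, passing each a LifeTime and marking it not in use.
; SpawnFromPool takes the first free one, moves it to the requested transform and flags it in use, without growing the pool.
; A ForLoopInDelay macro, not called here, runs loops in delayed batches, outputting row and column.
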(event Custom|InitalPool
  (for _index (range 0 (- (Variables|Default|GetPoolCount) 1))
    (bind _returnvalue (Game|SpawnActorfromClass (Variables|Default|GetPoolCharacter) (Math|Transform|MakeTransform "0.000000,0.000000,15000.000000" "0, 0, 0" "1.000000,1.000000,1.000000") "Undefined" "MultiplyWithRoot" 0 (Variables|Default|GetLife%20Time) 0))
    (Utilities|Array|AddUnique (Variables|Default|GetActorPools) _returnvalue)
    (Default|SetinUes _returnvalue false)))

(event EventBeginPlay
  (CallFunction|InitalPool))

(fn FindFirstAvailableActor
  (bind _array_element (Utilities|Array|ForEachLoopwithBreak (Variables|Default|GetActorPools) :!label _label)
    (:LoopBody
      (if (not (Variables|/Game/Blueprint/B_ObjectPool/BP_CharacterPool.BP_CharacterPool_C|GetInUse? _array_element))
        (Utilities|FlowControl|Sequence
          (:then_0
            (goto _label Break))
          (:then_1
            (return _array_element)))))))

(fn SpawnfromPool
  (params (ActorTransform :type Transform%20%28by%20ref%29))
  (bind _array_element (CallFunction|FindFirstAvailableActor))
  (Utilities|IsValid _array_element
    (:Is%20Valid
      (Transformation|SetActorTransform _array_element ActorTransform)
      (Default|SetinUes _array_element true)
      (return _array_element))))