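; Object pool component that pre-spawns actors of a configurable class on BeginPlay and reuses them in the game.
; SpawnFromPool takes the first actor not in use, moves it to the given transform and marks it in use, printing a message when none is free.
; A 分帧加载 (frame-split loading) macro, unused by the pool logic, runs loops in delayed batches and outputs row and column indices.
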(event Custom|InitalPool
  (for _index (range 0 (Variables|Default|GetPoolSize))
    (bind _returnvalue (Game|SpawnActorfromClass (Variables|Default|GetPoolActor) (Math|Transform|MakeTransform "0, 0, 0" "0, 0, 0" "1.000000,1.000000,1.000000") "Undefined" "MultiplyWithRoot" 0 0))
    (Utilities|Array|AddUnique (Variables|Default|GetObjectPool) _returnvalue)
    (Default|SetinUse _returnvalue false)))

(event EventBeginPlay
  (CallFunction|InitalPool))

(fn FindFirstAvailableActor
  (for _array_element (Variables|Default|GetObjectPool)
    (if (not (Variables|/Game/Blueprint/B_ObjectPool/BP_ActorPool.BP_ActorPool_C|GetInUse? _array_element))
      (return _array_element))))

(fn SpawnfromPool
  (params (Transforms :type Transform))
  (bind _poolactor (CallFunction|FindFirstAvailableActor))
  (Utilities|IsValid _poolactor
    (:Is%20Valid
      (Transformation|SetActorTransform _poolactor Transforms)
      (Default|SetinUse _poolactor true)
      (return _poolactor))
    (:Is%20Not%20Valid
      (Development|PrintString "Not Actor In Pool"))))