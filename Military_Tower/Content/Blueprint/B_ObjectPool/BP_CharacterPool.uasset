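; BP_CharacterPool is a poolable actor that toggles between an active and a dormant state instead of being destroyed, starting dormant on BeginPlay.
; SetInUes switches tick, collision and visibility together to match the in-use flag.
; When activated, it starts a LifeTime timer, clearing any previous one, that calls ReturnToPool to deactivate it again.
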(event Custom|SetInUes
  (params (InUse :type Boolean))
  (Variables|Default|SetInUse? InUse)
  (Actor|Tick|SetActorTickEnabled InUse)
  (Collision|SetActorEnableCollision InUse)
  (Rendering|SetActorHiddenInGame (not InUse))
  (Utilities|Time|ClearandInvalidateTimerbyHandle (Variables|Default|GetTimerHandle))
  (if InUse
    (bind _returnvalue (Utilities|Time|SetTimerbyEvent (delegate Custom|ReturnToPool) (Variables|Default|GetLifeTime)))
    (Variables|Default|SetTimerHandle _returnvalue)))

(event Custom|ReturnToPool
  (CallFunction|SetinUes false))

(event EventBeginPlay
  (CallFunction|SetinUes false))

(fn ConstructionScript)