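; BP_ActorPool is an actor that can be switched in and out of use for object pooling, starting inactive on BeginPlay.
; SetInUse stores the state, toggles collision, visibility and tick to match, and clears any running timer.
; Each activation starts a fresh timer that calls ReturnToPool after TimeToLive, deactivating the actor instead of destroying it.
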(event Custom|SetInUse
  (params (InUse? :type Boolean))
  (Variables|Default|SetInUse? InUse?)
  (Collision|SetActorEnableCollision InUse?)
  (Rendering|SetActorHiddenInGame (not InUse?))
  (Actor|Tick|SetActorTickEnabled InUse?)
  (Utilities|Time|ClearandInvalidateTimerbyHandle (Variables|Default|GetTimerHandle))
  (if InUse?
    (bind _returnvalue (Utilities|Time|SetTimerbyEvent (delegate Custom|ReturnToPool) (Variables|Default|GetTimeToLive)))
    (Variables|Default|SetTimerHandle _returnvalue)))

(event Custom|ReturnToPool
  (CallFunction|SetinUse false))

(event EventBeginPlay
  (CallFunction|SetinUse false))

(fn ConstructionScript)