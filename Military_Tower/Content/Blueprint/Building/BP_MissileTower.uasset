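; Missile tower building that lets the player place a missile target marker in the world with the mouse.
; Clicking either tower mesh while IsCoolDown is true spawns a BP_MissleTarget, enables input and starts a looping timer that snaps it to the cursor's visibility trace hit.
; A left click then fixes the target, pauses the timer and disables input; no firing or cooldown update happens here.
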(event OnClicked(StaticMesh)
  (params (TouchedComponent :type Primitive%20Component%20Object%20Reference) (ButtonPressed :type Key%20Structure))
  (if (Variables|Default|GetIsCoolDown?)
    (bind _returnvalue (Game|SpawnActorfromClass "/Game/Blueprint/Building/BP_MissleTarget.BP_MissleTarget_C" (Math|Transform|MakeTransform (.ImpactPoint (Collision|BreakHitResult (.HitResult (Game|Player|GetHitResultUnderCursorbyChannel (Game|GetPlayerController 0) "TraceTypeQuery1" true)))) "0, 0, 0" "2.000000,2.000000,2.000000") "Undefined" "MultiplyWithRoot" 0 0))
    (bind _output_get (Variables|Default|SetMissleTargetRef _returnvalue))
    (Utilities|IsValid _output_get
      (:Is%20Valid
        (Utilities|FlowControl|Sequence
          (:then_0
            (Variables|Default|SetIsMissleReady? true))
          (:then_1
            (bind _returnvalue_2 (Utilities|Time|SetTimerbyEvent (delegate Custom|TargetPointTrace) 0.016 true))
            (Variables|Default|SetTargetPointTraceHandle _returnvalue_2)
            (Utilities|FlowControl|DelayUntilNextFrame)
            (Input|EnableInput (Game|GetPlayerController 0)))))
      (:Is%20Not%20Valid
        (Utilities|Time|ClearandInvalidateTimerbyHandle (Variables|Default|GetTargetPointTraceHandle))))))

(event OnClicked(SM_Gun)
  (params (TouchedComponent :type Primitive%20Component%20Object%20Reference) (ButtonPressed :type Key%20Structure))
  (if (Variables|Default|GetIsCoolDown?)
    (bind _returnvalue (Game|SpawnActorfromClass "/Game/Blueprint/Building/BP_MissleTarget.BP_MissleTarget_C" (Math|Transform|MakeTransform (.ImpactPoint (Collision|BreakHitResult (.HitResult (Game|Player|GetHitResultUnderCursorbyChannel (Game|GetPlayerController 0) "TraceTypeQuery1" true)))) "0, 0, 0" "2.000000,2.000000,2.000000") "Undefined" "MultiplyWithRoot" 0 0))
    (bind _output_get (Variables|Default|SetMissleTargetRef _returnvalue))
    (Utilities|IsValid _output_get
      (:Is%20Valid
        (Utilities|FlowControl|Sequence
          (:then_0
            (Variables|Default|SetIsMissleReady? true))
          (:then_1
            (bind _returnvalue_2 (Utilities|Time|SetTimerbyEvent (delegate Custom|TargetPointTrace) 0.016 true))
            (Variables|Default|SetTargetPointTraceHandle _returnvalue_2)
            (Utilities|FlowControl|DelayUntilNextFrame)
            (Input|EnableInput (Game|GetPlayerController 0)))))
      (:Is%20Not%20Valid
        (Utilities|Time|ClearandInvalidateTimerbyHandle (Variables|Default|GetTargetPointTraceHandle))))))

(event Custom|TargetPointTrace
  (Transformation|SetActorLocation (Variables|Default|GetMissleTargetRef) (.ImpactPoint (Collision|BreakHitResult (.HitResult (Game|Player|GetHitResultUnderCursorbyChannel (Game|GetPlayerController 0) "TraceTypeQuery1" true)))) false false))

(event EventBeginPlay
  (|CallParentFunction) ; 此节点被禁用，将不会被调用。\n从引脚连出引线来编译功能。
)

(event Collision|EventActorBeginOverlap
  (params (OtherActor :type Actor%20Object%20Reference)))

(event EventTick
  (params (DeltaSeconds :type Float%20%28single-precision%29)))

(event Input|MouseEvents|LeftMouseButton
  (params (Key :type Key%20Structure))
  (:Pressed
    (if (Variables|Default|GetIsMissleReady?)
      (Transformation|SetActorLocation (Variables|Default|GetMissleTargetRef) (.ImpactPoint (Collision|BreakHitResult (.HitResult (Game|Player|GetHitResultUnderCursorbyChannel (Game|GetPlayerController 0) "TraceTypeQuery1" true)))) false false)
      (Utilities|Time|PauseTimerbyHandle (Variables|Default|GetTargetPointTraceHandle))
      (Variables|Default|SetIsMissleReady? false)
      (Utilities|FlowControl|DelayUntilNextFrame)
      (Input|DisableInput (Game|GetPlayerController 0)))))

(fn ConstructionScript
  (|CallParentFunction))