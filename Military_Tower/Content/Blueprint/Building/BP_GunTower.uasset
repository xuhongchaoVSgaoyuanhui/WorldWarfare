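; BP_GunTower is a gun tower building that turns its gun mesh toward a nearby enemy.
; A looping timer smoothly interpolates the rotation, unpausing and pausing as that enemy enters and leaves the detection sphere.
; On BeginPlay it checks whether the nearest BP_Radar is within a fixed distance.
; Radar coverage lifts the rotation angle limit that otherwise constrains the gun.
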(event OnComponentBeginOverlap(Sphere)
  (params (OverlappedComponent :type Primitive%20Component%20Object%20Reference) (OtherActor :type Actor%20Object%20Reference) (OtherComp :type Primitive%20Component%20Object%20Reference) (OtherBodyIndex :type Integer) (bFromSweep :type Boolean) (SweepResult :type Hit%20Result%20Structure%20%28by%20ref%29))
  (if (== OtherActor (CallFunction|FindNearEnemy))
    (Utilities|Time|UnpauseTimerbyHandle (Variables|Default|GetGunRotateHandleTimer))))

(event OnComponentEndOverlap(Sphere)
  (params (OverlappedComponent :type Primitive%20Component%20Object%20Reference) (OtherActor :type Actor%20Object%20Reference) (OtherComp :type Primitive%20Component%20Object%20Reference) (OtherBodyIndex :type Integer))
  (if (== OtherActor (CallFunction|FindNearEnemy))
    (Utilities|Time|PauseTimerbyHandle (Variables|Default|GetGunRotateHandleTimer))))

(event Custom|RotateToEnemy
  (bind _sm_gun (Variables|Default|GetSM_Gun))
  (bind _sm_gun_2 (Variables|Default|GetSM_Gun))
  ;[0 0 0] 控制机枪旋转朝向敌人
  (bind _enemyloc (Class|InterfaceEnemyLoc|GetEnemyLocation(Message) (CallFunction|FindNearEnemy)))
  (if (stale EventBeginPlay _isincludeinarea)
    (Transformation|SetWorldRotation _sm_gun_2 (Math|Interpolation|RInterpTo (Transformation|GetWorldRotation _sm_gun) (Math|Rotator|FindLookatRotation (Transformation|GetWorldLocation _sm_gun) _enemyloc) (Utilities|Time|GetWorldDeltaSeconds) 5.0) false false)
    (else
      (Transformation|SetWorldRotation _sm_gun_2 (CallFunction|LimitGunRotateAngle (Math|Interpolation|RInterpTo (Transformation|GetWorldRotation _sm_gun) (Math|Rotator|FindLookatRotation (Transformation|GetWorldLocation _sm_gun) _enemyloc) (Utilities|Time|GetWorldDeltaSeconds) 5.0)) false false))))

(event EventBeginPlay
  (|CallParentFunction)
  ;[0 0 0 0.5] 检测雷达防御塔是否在附近
  (bind _outactors (Actor|GetAllActorsOfClass "/Game/Blueprint/Building/BP_Radar.BP_Radar_C"))
  (Utilities|IsValid (.ReturnValue (Actor|FindNearestActor (Transformation|GetActorLocation) _outactors))
    (:Is%20Valid
      (bind _isincludeinarea (CallFunction|CalculateNearestRadarTowerorNot (.ReturnValue (Actor|FindNearestActor (Transformation|GetActorLocation) _outactors)))))
    (:Is%20Not%20Valid
      _))
  ;[0 0 0] 控制机枪旋转朝向敌人
  (bind _returnvalue (Utilities|Time|SetTimerbyEvent (delegate Custom|RotateToEnemy) 0.03 true))
  (Variables|Default|SetGunRotateHandleTimer _returnvalue)
  (Utilities|FlowControl|DelayUntilNextTick)
  (Utilities|Time|PauseTimerbyHandle (Variables|Default|GetGunRotateHandleTimer)))

(fn ConstructionScript
  (|CallParentFunction))

(fn CalculateNearestRadarTowerorNot
  (params (RadarActor :type Actor%20Object%20Reference))
  (return (<= (Math|Vector|Distance(Vector) (Transformation|GetActorLocation RadarActor) (Transformation|GetActorLocation)) 1.8e+03)))