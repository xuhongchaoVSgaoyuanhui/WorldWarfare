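; BP_MainBuild is a building Blueprint that populates an instanced static mesh at BeginPlay.
; It loops over a fixed index range, adds world-space instances from the InstanceTransform array and prints each returned instance index.
; A helper function returns the world location of an instance by index; despite its TransformUpdate name, it only reads the transform.
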(event EventBeginPlay
  (for _index (range 0 8)
    (bind _returnvalue (Components|InstancedStaticMesh|AddInstance (Variables|Default|GetInstancedStaticMesh) (Utilities|Array|Get(acopy) (Variables|Default|GetinstanceTransform) _index) true))
    (Development|PrintString (Utilities|String|ToString(Integer) _returnvalue))))

(event Collision|EventActorBeginOverlap
  (params (OtherActor :type Actor%20Object%20Reference)))

(event EventTick
  (params (DeltaSeconds :type Float%20%28single-precision%29)))

(fn ConstructionScript)

(fn FUTransformUpdateBaseLocationInt
  (params (Instance%20Index :type Integer))
  (return (.location (.OutInstanceTransform (Components|InstancedStaticMesh|GetInstanceTransform (Variables|Default|GetInstancedStaticMesh) Instance%20Index true)))))