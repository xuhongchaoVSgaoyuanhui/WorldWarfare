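; Base tower Blueprint that provides enemy lookup and gun rotation limiting for defensive towers.
; On BeginPlay it async-loads a soft-referenced enemy spawner, caches it and copies its enemy array once, if not empty.
; FindNearEnemy returns the closest actor from that copy, and LimitGunRotateAngle clamps yaw within a set angle either side of the Arrow's facing.
; A deprecated, disconnected branch loads enemy base assets.
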(event EventBeginPlay
  (bind _object (Utilities|AsyncLoadAsset (Variables|Default|GetEnemySpawnerSoftRef))
    (:Completed
      (bind _asbp_enemy_spawner (Utilities|Casting|CastToBP_EnemySpawner _object))
      (Utilities|IsValid _asbp_enemy_spawner
        (:Is%20Valid
          (bind _output_get (Variables|Default|SetEnemyspawner _asbp_enemy_spawner))
          (if (not (Utilities|Array|IsEmpty (Variables|/Game/Blueprint/B_Enemy/BP_EnemySpawner.BP_EnemySpawner_C|GetEnemyArray _output_get)))
            (Variables|Default|SetAllEnemy (Variables|/Game/Blueprint/B_Enemy/BP_EnemySpawner.BP_EnemySpawner_C|GetEnemyArray _output_get))))))))

(fn ConstructionScript)

(fn FindNearEnemy
  (return (.ReturnValue (Actor|FindNearestActor (Transformation|GetActorLocation) (Variables|Default|GetAllEnemy)))))

(fn LimitGunRotateAngle
  (params (InRot :type Rotator))
  (bind (_roll _pitch _yaw) (Math|Rotator|BreakRotator InRot))
  (bind _arrow (Variables|Default|GetArrow))
  (bind _m_limitangle (LocalVariables|Getm_LimitAngle))
  (bind _returnvalue (Transformation|GetWorldRotation _arrow))
  (return (Math|Rotator|MakeRotator _roll _pitch (Math|Float|ClampAngle _yaw (- (.yaw _returnvalue) _m_limitangle) (+ (.yaw _returnvalue) _m_limitangle)))))