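; BP_Radar is a radar building whose SMGun component spins continuously and turns faster when an enemy comes within range.
; A looping timer started on BeginPlay repeatedly adds RadarRotateAngle as a relative rotation to SMGun.
; Sphere overlap events raise that angle when the actor returned by FindNearEnemy enters and lower it when that actor leaves.
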(event OnComponentBeginOverlap(Sphere)
  (params (OverlappedComponent :type Primitive%20Component%20Object%20Reference) (OtherActor :type Actor%20Object%20Reference) (OtherComp :type Primitive%20Component%20Object%20Reference) (OtherBodyIndex :type Integer) (bFromSweep :type Boolean) (SweepResult :type Hit%20Result%20Structure%20%28by%20ref%29))
  (if (== OtherActor (CallFunction|FindNearEnemy))
    (Variables|Default|SetRadarRotateAngle "0.000000,10.000000,0.000000")))

(event OnComponentEndOverlap(Sphere)
  (params (OverlappedComponent :type Primitive%20Component%20Object%20Reference) (OtherActor :type Actor%20Object%20Reference) (OtherComp :type Primitive%20Component%20Object%20Reference) (OtherBodyIndex :type Integer))
  (if (== OtherActor (CallFunction|FindNearEnemy))
    (Variables|Default|SetRadarRotateAngle "0.000000,3.000000,0.000000")))

(event Custom|AddRadarRorateAngle
  (Transformation|AddRelativeRotation (Variables|Default|GetSM_Gun) (Variables|Default|GetRadarRotateAngle) false false))

(event EventBeginPlay
  (|CallParentFunction)
  (Utilities|Time|SetTimerbyEvent (delegate Custom|AddRadarRorateAngle) 0.03 true))

(fn ConstructionScript
  (|CallParentFunction))