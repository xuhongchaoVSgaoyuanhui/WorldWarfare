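; Defensive tower whose machine-gun type turns its gun mesh to face an enemy inside its detection sphere.
; BeginPlay caches a single BP_Enemy and, for that type, creates a paused looping timer that smoothly interpolates the gun toward the enemy's location, fetched by interface message.
; Sphere overlaps with that enemy resume or pause the timer, resetting world rotation on exit.
; No firing logic exists; the construction script's type switch is empty.
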(event OnComponentBeginOverlap(Sphere)
  (params (OverlappedComponent :type Primitive%20Component%20Object%20Reference) (OtherActor :type Actor%20Object%20Reference) (OtherComp :type Primitive%20Component%20Object%20Reference) (OtherBodyIndex :type Integer) (bFromSweep :type Boolean) (SweepResult :type Hit%20Result%20Structure%20%28by%20ref%29))
  (if (== OtherActor (Variables|Default|GetEnemyRef))
    (Utilities|Time|UnpauseTimerbyHandle (Variables|Default|GetRotateHandleTimer))))

(event OnComponentEndOverlap(Sphere)
  (params (OverlappedComponent :type Primitive%20Component%20Object%20Reference) (OtherActor :type Actor%20Object%20Reference) (OtherComp :type Primitive%20Component%20Object%20Reference) (OtherBodyIndex :type Integer))
  (if (== (Variables|Default|GetEnemyRef) OtherActor)
    (Utilities|Time|PauseTimerbyHandle (Variables|Default|GetRotateHandleTimer))
    (Utilities|FlowControl|DelayUntilNextTick)
    (Transformation|SetWorldRotation (Variables|Default|GetSM_Gun) "0, 0, 0" false false)))

(event Custom|RotateToEnemy
  (bind _sm_gun (Variables|Default|GetSM_Gun))
  (bind _enemyloc (Class|InterfaceEnemyLoc|GetEnemyLocation(Message) (Variables|Default|GetEnemyRef)))
  (Transformation|SetWorldRotation (Variables|Default|GetSM_Gun) (Math|Interpolation|RInterpTo (Transformation|GetWorldRotation _sm_gun) (Math|Rotator|FindLookatRotation (Transformation|GetWorldLocation _sm_gun) _enemyloc) (Utilities|Time|GetWorldDeltaSeconds) 5.0) false false))

(event EventBeginPlay
  (bind _returnvalue (Actor|GetActorOfClass "/Game/Blueprint/Enemy/BP_Enemy.BP_Enemy_C"))
  (Variables|Default|SetEnemyRef _returnvalue)
  (switch Utilities|FlowControl|Switch|SwitchonE_TowerType (Variables|Default|GetTowerType)
    (:NewEnumerator0
      (bind _returnvalue_2 (Utilities|Time|SetTimerbyEvent (delegate Custom|RotateToEnemy) 0.02 true))
      (Variables|Default|SetRotateHandleTimer _returnvalue_2)
      (Utilities|FlowControl|DelayUntilNextTick)
      (Utilities|Time|PauseTimerbyHandle (Variables|Default|GetRotateHandleTimer)))))

(fn ConstructionScript
  (switch Utilities|FlowControl|Switch|SwitchonE_TowerType (Variables|Default|GetTowerType)))