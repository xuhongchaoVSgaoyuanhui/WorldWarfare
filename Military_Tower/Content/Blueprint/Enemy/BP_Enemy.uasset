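; BP_Enemy is an enemy pawn that walks along a referenced BPEnemySpline point by point.
; From BeginPlay, MoveTo runs AI MoveTo to the current spline point and, on success, waits briefly, increments the index and calls itself again.
; The index has no end or wrap check, failed moves are not retried, and a missing spline only prints a message.
; GetEnemyLocation exposes the actor's location.
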(event Custom|MoveTo
  (Utilities|IsValid (Variables|Default|Get%20BP_EnemySpline)
    (:Is%20Valid
      (AI|AIMoveTo self (Spline|GetLocationatSplinePoint (Variables|/Game/Blueprint/Enemy/BP_EnemySpline.BP_EnemySpline_C|GetSpline (Variables|Default|Get%20BP_EnemySpline)) (Variables|Default|GetSpline%20Point%20Index) "World") 0 5.0 false
        (:OnSuccess
          (Utilities|FlowControl|Delay 0.1)
          (Math|Integer|IncrementInt (Variables|Default|GetSpline%20Point%20Index)
            (:%20%20
              (CallFunction|Moveto))))))
    (:Is%20Not%20Valid
      (Development|PrintString "NO Spline "))))

(event EventBeginPlay
  (CallFunction|Moveto))

(fn ConstructionScript)

(fn GetEnemyLocation
  (return (Transformation|GetActorLocation)))