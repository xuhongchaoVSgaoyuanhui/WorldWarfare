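; Base enemy pawn that walks along an assigned spline path using AI navigation.
; MoveTo steps through spline points, picking a random reachable point near each and recursing after a short random delay on success.
; On BeginPlay it caches all towers and their locations for a nearest-tower lookup.
; The construction script sizes the attack range sphere from AttackRange; perception currently only prints sensed actors.
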(event OnPerceptionUpdated(AIPerception)
  (params (UpdatedActors :type Array%20of%20Actor%20Object%20References)))

(event OnTargetPerceptionUpdated(AIPerception)
  (params (Actor :type Actor%20Object%20Reference) (Stimulus :type AI%20Stimulus%20Structure))
  (if (.bSuccessfullySensed (Utilities|Struct|BreakAIStimulus Stimulus))
    (Development|PrintString (Utilities|GetDisplayName Actor))))

(event Custom|MoveTo
  (Utilities|IsValid (Variables|Default|Get%20BP_EnemySpline)
    (:Is%20Valid
      (AI|AIMoveTo self (.RandomLocation (AI|Navigation|GetRandomReachablePointinRadius (Spline|GetLocationatSplinePoint (Variables|/Game/Blueprint/Enemy/BP_EnemySpline.BP_EnemySpline_C|GetSpline (Variables|Default|Get%20BP_EnemySpline)) (Variables|Default|GetSpline%20Point%20Index) "World") 1e+02 0 0)) 0 5.0 false
        (:OnSuccess
          (Utilities|FlowControl|Delay (Math|Random|RandomFloatinRange 0.0 0.1))
          (Math|Integer|IncrementInt (Variables|Default|GetSpline%20Point%20Index)
            (:%20%20
              (CallFunction|Moveto))))))
    (:Is%20Not%20Valid
      (Development|PrintString "NO Spline "))))

(event EventBeginPlay
  (bind _outactors (Actor|GetAllActorsOfClass "/Game/Blueprint/Building/BP_TowerBase.BP_TowerBase_C"))
  (bind _output_get (Variables|Default|SetAllTowers _outactors))
  (for _array_element _output_get
    (Utilities|Array|AddUnique (Variables|Default|GetAllTowerLocations) (Transformation|GetActorLocation _array_element))))

(fn ConstructionScript
  (Components|Sphere|SetSphereRadius (Variables|Default|GetAtkRangeSphere) (* (Variables|攻击|GetAttackRange) 5.0) true))

(fn GetNeatesTower
  (return (.ReturnValue (Actor|FindNearestActor (Transformation|GetActorLocation) (Variables|Default|GetAllTowers)))))

(fn GetEnemyLocation
  (return (Transformation|GetActorLocation)))