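; Enemy soldier Blueprint that begins moving on spawn and tracks whether its nearest tower is within attack range, relying on a parent class.
; BeginPlay runs the parent logic, then calls MoveTo.
; AtkRangeSphere overlaps set or clear CanAttack when the other actor matches the tower returned by GetNeatesTower.
; Attack and Tick are empty here, and the NSFires effect toggles are unconnected.
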(event OnComponentBeginOverlap(AtkRangeSphere)
  (params (OverlappedComponent :type Primitive%20Component%20Object%20Reference) (OtherActor :type Actor%20Object%20Reference) (OtherComp :type Primitive%20Component%20Object%20Reference) (OtherBodyIndex :type Integer) (bFromSweep :type Boolean) (SweepResult :type Hit%20Result%20Structure%20%28by%20ref%29))
  (if (== OtherActor (CallFunction|GetNeatesTower))
    (Variables|Default|SetCanAttack? true)))

(event OnComponentEndOverlap(AtkRangeSphere)
  (params (OverlappedComponent :type Primitive%20Component%20Object%20Reference) (OtherActor :type Actor%20Object%20Reference) (OtherComp :type Primitive%20Component%20Object%20Reference) (OtherBodyIndex :type Integer))
  (if (== (CallFunction|GetNeatesTower) OtherActor)
    (Variables|Default|SetCanAttack? false)))

(event Custom|Attack)

(event EventBeginPlay
  (|CallParentFunction)
  (CallFunction|Moveto))

(event EventTick
  (params (DeltaSeconds :type Float%20%28single-precision%29)))

(fn ConstructionScript
  (|CallParentFunction))