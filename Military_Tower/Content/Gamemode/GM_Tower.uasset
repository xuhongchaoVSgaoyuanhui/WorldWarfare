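; GM_Tower is the game mode for a tower game, handling start-up on BeginPlay.
; It checks whether the BP_Camera player pawn has a command center, calling the still-empty FUGamePlay if so or printing a prompt to place one.
; It then spawns a BP_TimerManager and stores the reference on GS_Tower, the game state.
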(event EventBeginPlay
  (CallFunction|FUGameStart)
  (bind _returnvalue (Game|SpawnActorfromClass "/Game/Blueprint/BP_TimerManager.BP_TimerManager_C" (Math|Transform|MakeTransform "0, 0, 0" "0, 0, 0" "1.000000,1.000000,1.000000") "AlwaysSpawn" "MultiplyWithRoot" 0 0))
  (bind _asgs_tower (Utilities|Casting|CastToGS_Tower (Game|GetGameState)))
  (Variables|/Game/Gamemode/GS_Tower.GS_Tower_C|SetTimerManager _asgs_tower _returnvalue))

(event EventTick
  (params (DeltaSeconds :type Float%20%28single-precision%29)))

(fn ConstructionScript)

(fn FUGameStart
  (bind _asbp_camera (Utilities|Casting|CastToBP_Camera (Game|Player|GetPlayerPawn 0)))
  (if (Variables|/Game/Blueprint/B_Pawn/BP_Camera.BP_Camera_C|GetishasCommand _asbp_camera)
    (CallFunction|FUGamePlay)
    (else
      (Development|PrintString "请放置指挥中心" true true "(R=1.000000,G=0.100937,B=0.090433,A=1.000000)" 2e+03))))

(fn FUGamePlay)