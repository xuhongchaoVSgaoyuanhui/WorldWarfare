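; Player controller for the Tower game mode that moves the pawn through Enhanced Input and detects objects under the mouse cursor.
; On BeginPlay it adds the mapping context and registers a looping timer by name with a custom FU timer manager, which the code notes is discouraged outside special classes.
; The timer runs a cursor line trace, messaging hit actors with the hit item index.
; Debug keys pause, resume, clear and query timers.
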(event Input|EnhancedActionEvents|EnhancedInputActionIA_Move
  (params (ActionValue :type Vector%202D%20Structure) (ElapsedSeconds :type Float%20%28double-precision%29) (TriggeredSeconds :type Float%20%28double-precision%29) (InputAction :type Input%20Action%20Object%20Reference :default "/Game/Input/IA_Move.IA_Move"))
  (bind _returnvalue (Game|Player|GetPlayerPawn 0))
  (Pawn|Input|AddMovementInput _returnvalue (Transformation|GetActorForwardVector _returnvalue) (.x ActionValue) true)
  (Pawn|Input|AddMovementInput (Game|Player|GetPlayerPawn 0) (Transformation|GetActorRightVector _returnvalue) (.y ActionValue) true))

(event EventBeginPlay
  (bind _self self)
  (bind _returnvalue (PlayerController|LocalPlayerSubsystems|GetEnhancedInputLocalPlayerSubsystem _self))
  (Utilities|IsValid _returnvalue
    (:Is%20Valid
      (Input|AddMappingContext _returnvalue "/Game/Input/IMC_Tower.IMC_Tower" 0 "(bIgnoreAllPressedKeysUntilRelease=True,bForceImmediately=False,bNotifyUserSettings=False)")
      (bind _output_get (Variables|Default|SetTimerManager (CallFunction|FUGetTimerManager)))
      ;[1 0.6403 0] 注册定时器，不推荐此操作，仅限于单独特定类，其他所有类使用定时器，请使用FU_RegisterEventTimerCallback
      (Development|PrintString "注册定时器" true true "(R=1.000000,G=0.658285,B=0.243454,A=1.000000)" 1e+01)
      (Class|InterfaceTimerEntry|FURegisterTimer(Message) _output_get self "FU_vector3LineTraceDetection" 0.05 true))))

(event Input|KeyboardEvents|Q
  (params (Key :type Key%20Structure :default "None"))
  (:Pressed
    (Development|PrintString "清除定时器" true true "(R=1.000000,G=0.000000,B=0.234128,A=1.000000)" 1e+01)
    (Class|InterfaceTimerEntry|FUClearAssignTimer(Message) (Variables|Default|GetTimerManager) "FU_vector3LineTraceDetection")))

(event Input|KeyboardEvents|E
  (params (Key :type Key%20Structure :default "None"))
  (bind _timermanager (Variables|Default|GetTimerManager))
  (:Pressed
    (Utilities|FlowControl|FlipFlop
      (:A
        (Development|PrintString "执行暂停定时器函数" true true "(R=0.789619,G=0.000000,B=1.000000,A=1.000000)" 1e+01)
        (Class|InterfaceTimerEntry|FUPauseAssignTimer(Message) _timermanager "FU_vector3LineTraceDetection"))
      (:B
        (Development|PrintString "继续被暂停定时器函数" true true "(R=0.139727,G=1.000000,B=0.039125,A=1.000000)" 1e+01)
        (Class|InterfaceTimerEntry|FUUnpauseAssignTimer(Message) _timermanager "FU_vector3LineTraceDetection")))))

(event Input|KeyboardEvents|1
  (params (Key :type Key%20Structure :default "None"))
  (:Pressed
    (Development|PrintString "查询整个场景中已经注册的定时器.........." true true "(R=1.000000,G=0.182194,B=0.646576,A=1.000000)" 2e+02)
    (Utilities|FlowControl|Delay 2.0)
    (Default|FU111 (CallFunction|FUGetTimerManager))))

(fn ConstructionScript)

(fn FUVector3LineTraceDetection
  (bind (_worldlocation _worlddirection) (Game|Player|ConvertMouseLocationToWorldSpace))
  (bind (_outhit _returnvalue) (Collision|LineTraceForObjects _worldlocation (+ _worldlocation (* _worlddirection 20000)) (Utilities|Array|MakeArray "ObjectTypeQuery7") false 0 "ForDuration"))
  (if _returnvalue
    (Class|InterfaceBuildingplacement|FUTransformUpdateBaseLocationInt(Message) (.HitActor (Collision|BreakHitResult _outhit)) (.HitItem (Collision|BreakHitResult _outhit)))
    (return)))

(fn PCTowerAutoGenFunc)