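; BP_GamePawn is a pawn whose spring arm length the player adjusts through input, zooming in and out.
; On BeginPlay it adds the IMC_Player mapping context to the first player controller's Enhanced Input subsystem.
; The IA_UpOrDown action scales its value and adds it to the arm length, clamped to a fixed range, and prints a debug string each trigger.
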(event Input|EnhancedActionEvents|EnhancedInputActionIA_UpOrDown
  (params (ActionValue :type Float%20%28double-precision%29) (ElapsedSeconds :type Float%20%28double-precision%29) (TriggeredSeconds :type Float%20%28double-precision%29) (InputAction :type Input%20Action%20Object%20Reference :default "/Game/feishi/Input/IA_UpOrDown.IA_UpOrDown"))
  (bind _springarm (Variables|Default|GetSpringArm))
  (:Triggered
    (Development|PrintString "Hello")
    (Variables|/Script/Engine.SpringArmComponent|SetTargetArmLength _springarm (Math|Float|Clamp(Float) (+ (Variables|/Script/Engine.SpringArmComponent|GetTargetArmLength _springarm) (* ActionValue 1e+02)) 1.5e+03 3e+03))))

(event EventBeginPlay
  (Input|AddMappingContext (PlayerController|LocalPlayerSubsystems|GetEnhancedInputLocalPlayerSubsystem (Game|GetPlayerController 0)) "/Game/feishi/Input/IMC_Player.IMC_Player" 0 "(bIgnoreAllPressedKeysUntilRelease=True,bForceImmediately=False,bNotifyUserSettings=False)"))

(fn ConstructionScript)